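; BP_Pickup is a power-up pickup that unlocks an ability for the third-person character.
; When that character overlaps its sphere, a switch on PowerUpToUnlock grants special attack, an extra jump or sprint, then destroys the pickup.
; The construction script picks the static mesh from the same setting, though the Sprint option has no mesh assigned.
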(event `self.Sphere.OnComponentBeginOverlap`
  (params (OverlappedComponent :type "PrimitiveComponent Object Reference") (OtherActor :type "Actor Object Reference") (OtherComp :type "PrimitiveComponent Object Reference") (OtherBodyIndex :type Integer) (bFromSweep :type Boolean) (SweepResult :type "HitResult Structure (by ref)"))
  (bind _asbp_third_person_character (cast `/Game/Blueprints/BP_ThirdPersonCharacter` OtherActor))
  (switch `/Game/Blueprints/EPowerUps` (`self.PowerUpToUnlock`)
    (:`NewEnumerator0`
      (set `/Game/Blueprints/BP_ThirdPersonCharacter.HasSpecialAttack` true _asbp_third_person_character)
      (`self.K2_DestroyActor`))
    (:`NewEnumerator1`
      (`/Game/Blueprints/BP_ThirdPersonCharacter.AddJumpCount` _asbp_third_person_character)
      (`self.K2_DestroyActor`))
    (:`NewEnumerator2`
      (set `/Game/Blueprints/BP_ThirdPersonCharacter.HasSprint` true _asbp_third_person_character)
      (`self.K2_DestroyActor`))))

(fn `UserConstructionScript`
  (`StaticMeshComponent.SetStaticMesh` (`self.StaticMesh`) (select `/Game/Blueprints/EPowerUps` (`self.PowerUpToUnlock`) :`NewEnumerator0` "/Game/Assets/Props/Powerups/Powerup_A/SM_Powerup_A.SM_Powerup_A" :`NewEnumerator1` "/Game/Assets/Props/Collectibles/Common/SM_Collectible_Common.SM_Collectible_Common" :!type "StaticMesh Object Reference")))